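; Intro cutscene actor that plays a queue of Level Sequences with subtitles, switching to the cinematic character and back.
; Each step creates a sequence player with its LoopCollection loop count and shows the matching data table line in WB_Subtitles.
; Non-infinite sequences pause just before their end time.
; Finishing or a press-to-continue skip advances the queue; after the last entry it removes subtitles, switches character and destroys itself.
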(event `Next Cutscene`
  (bind _output (`|GetArrayItem` (`self.LoopCollection`) (`self.LoopQueue`)))
  (bind _returnvalue (!= _output -1))
  ;[1 1 1] Сцены
  (bind _outactor (`LevelSequencePlayer.CreateLevelSequencePlayer` (`|GetArrayItem` (`self.StartingSequence`) (`self.SequenceCutsceneNum`))))
  (`self.Showtext`)
  (bind _sequenceplayer (`LevelSequenceActor.SequencePlayer` _outactor))
  ;[1 1 1] Цикл катсцены
  (`MovieSceneSequencePlayer.PlayLooping` _sequenceplayer _output)
  (if _returnvalue
    (`KismetSystemLibrary.Delay` (- (`TimeManagementBlueprintLibrary.Conv_QualifiedFrameTimeToSeconds` (`MovieSceneSequencePlayer.GetEndTime` _sequenceplayer)) 0.05))
    (if _returnvalue
      (`MovieSceneSequencePlayer.Pause` _sequenceplayer)
      (add `MovieSceneSequencePlayer.OnFinished` _sequenceplayer (delegate `Finished anim`) :!label _label))
    (else
      (goto _label))))

(event `self.ReceiveBeginPlay`
  (`self.createSubtitles`)
  ;[1 1 1] gameCharacter
  (bind _asgame_controller (cast `/Game/Controllers/GameController` (`GameplayStatics.GetPlayerController` 0)))
  (`/Game/Controllers/GameController.ChangeCharacter` _asgame_controller)
  (bind _ascinamatic_character (cast `/Game/BP_Characters/CinamaticCharacter` (`GameplayStatics.GetPlayerCharacter` 0)))
  (bind _output_get (set `self.As Cinamatic Character` _ascinamatic_character))
  (`self.Next Cutscene`)
  (add `/Game/BP_Characters/CinamaticCharacter.PressToContinue` _output_get (delegate `PressToContinue_Event`)))

(event `Finished anim`
  ;[1 1 1] Цикл катсцены
  (if (!= (`KismetArrayLibrary.Array_Length` (`self.LoopCollection`)) (+ (`self.LoopQueue`) 1))
    ;[1 1 1] nextCutscene
    (bind _result (`/Engine/EditorBlueprintResources/StandardMacros.IncrementInt` (`self.LoopQueue`))
      (:`  `
        (set `self.LoopQueue` _result)
        (bind _result_2 (`/Engine/EditorBlueprintResources/StandardMacros.IncrementInt` (`self.SequenceCutsceneNum`))
          (:`  `
            (set `self.SequenceCutsceneNum` _result_2)
            (bind _result_3 (`/Engine/EditorBlueprintResources/StandardMacros.IncrementInt` (`self.CurrentText`))
              (:`  `
                (set `self.CurrentText` _result_3)
                (`/Game/UI/WB_Subtitles.EmptyText` (`self.SubtitlesWidgetRef`))
                (`self.Next Cutscene`)))))))
    (else
      ;[1 1 1] End of scene
      (`self.HideText`)
      (bind _asgame_controller (cast `/Game/Controllers/GameController` (`GameplayStatics.GetPlayerController` 0)))
      (`/Game/Controllers/GameController.ChangeCharacter` _asgame_controller)
      (`self.K2_DestroyActor`))))

(event `createSubtitles`
  (bind _returnvalue (`|CreateWidget` "/Game/UI/WB_Subtitles.WB_Subtitles_C"))
  (bind _output_get (set `self.SubtitlesWidgetRef` _returnvalue))
  (`UserWidget.AddToViewport` _output_get 0)
  (`self.ClearSubtitles`))

(event `ClearSubtitles`
  (`/Game/UI/WB_Subtitles.DisplayLine` (`self.SubtitlesWidgetRef`) ""))

(event `PressToContinue_Event`
  ;[1 1 1] Пропуск кат сцены
  (`MovieSceneSequencePlayer.GoToEndAndStop` (`LevelSequenceActor.SequencePlayer` (stale `Next Cutscene` _outactor)))
  (set `self.Action Button is pressed` true)
  (`self.Finished anim`))

(event `hideTextBox_Event`
  (`Widget.RemoveFromParent` (`self.SubtitlesWidgetRef`)))

(event `ShowNextLine`
  (params (NarrationList :type "DataTable Object Reference"))
  (bind _currentnarrationlist (`self.CurrentNarrationList`))
  (set `self.CurrentNarrationList` NarrationList)
  (bind _outrownames (`DataTableFunctionLibrary.GetDataTableRowNames` _currentnarrationlist))
  (bind _returnvalue (`|GetDataTableRow` _currentnarrationlist (`|GetArrayItem` _outrownames (`self.CurrentText`)))
    (:`then`
      (`/Game/UI/WB_Subtitles.DisplayLine` (`self.SubtitlesWidgetRef`) (`.LineToShow_3_12BE9ADF4F9B936B8326BBAABD50D48D` (break `/Game/TextInGame/SubtitlesStruct` _returnvalue))))))

(event `Showtext`
  ;[1 1 1] show text
  (`self.ShowNextLine` (`self.TextCollection`)))

(event `HideText`
  (`Widget.RemoveFromParent` (`self.SubtitlesWidgetRef`)))

(fn `UserConstructionScript`)