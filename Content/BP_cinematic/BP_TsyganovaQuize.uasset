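; Quiz encounter actor (Tsyganova): overlap boxes show a name label and an interact prompt, and talking starts a cutscene-driven quiz.
; Skippable level sequences with data-table subtitles chain on finish events, then hand off to a timed, scored quiz widget.
; The score picks a good or bad ending sequence; good saves a point and leaves only completion dialogue for later talks.
; GameController dispatchers drive talk, skip, timeout and score-screen exit.
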(event `self.Box.OnComponentBeginOverlap`
  (params (OverlappedComponent :type "PrimitiveComponent Object Reference") (OtherActor :type "Actor Object Reference") (OtherComp :type "PrimitiveComponent Object Reference") (OtherBodyIndex :type Integer) (bFromSweep :type Boolean) (SweepResult :type "HitResult Structure (by ref)"))
  ;[1 1 1] Overlaptheactor
  (bind _returnvalue (`|CreateWidget` "/Game/UI/WP_Interact.WP_Interact_C"))
  (bind _output_get (set `self.InteractOption` _returnvalue))
  (`UserWidget.AddToViewport` _output_get 0)
  (`/Game/UI/WP_Interact.StartInteract` _output_get)
  (bind _asgame_controller (cast `/Game/Controllers/GameController` (`GameplayStatics.GetPlayerController` 0)))
  (add `/Game/Controllers/GameController.StartTheTalk` _asgame_controller (delegate `StartTheMainScript`)))

(event `Next Cutscene`
  (params (isEnding :type Boolean) (EndingCutscene :type "LevelSequenceActor Object Reference") (Looping :type Integer))
  (bind _sequence_player (`self.Sequence Player`))
  (bind _output (`|GetArrayItem` (`self.LoopCollection`) (`self.LoopQueue`)))
  (bind _returnvalue (!= _output -1))
  ;[1 1 1] Сцены
  (if isEnding
    (set `self.LoopingEnding` Looping)
    (set `self.Sequence Player` (`LevelSequenceActor.SequencePlayer` EndingCutscene))
    (else
      (bind _outactor (`LevelSequencePlayer.CreateLevelSequencePlayer` (`|GetArrayItem` (`self.StartingSequence`) (`self.SequenceCutsceneNum`))))
      (`self.Showtext` false)
      (set `self.Sequence Player` (`LevelSequenceActor.SequencePlayer` _outactor))))
  ;[1 1 1] Цикл катсцены
  (if (`self.IsQuizOn`)
    (`MovieSceneSequencePlayer.PlayLooping` _sequence_player _output)
    (else
      (`MovieSceneSequencePlayer.PlayLooping` _sequence_player (`self.LoopingEnding`))))
  (if _returnvalue
    (`KismetSystemLibrary.Delay` (- (`TimeManagementBlueprintLibrary.Conv_QualifiedFrameTimeToSeconds` (`MovieSceneSequencePlayer.GetEndTime` _sequence_player)) 0.05))
    (if _returnvalue
      (`MovieSceneSequencePlayer.Pause` _sequence_player)
      (add `MovieSceneSequencePlayer.OnFinished` _sequence_player (delegate `Finished anim`) :!label _label))
    (else
      (goto _label))))

(event `self.Box.OnComponentEndOverlap`
  (params (OverlappedComponent :type "PrimitiveComponent Object Reference") (OtherActor :type "Actor Object Reference") (OtherComp :type "PrimitiveComponent Object Reference") (OtherBodyIndex :type Integer))
  (bind _interactoption (`self.InteractOption`))
  ;[1 1 1] Overlaptheactor
  (`/Engine/EditorBlueprintResources/StandardMacros.IsValid` _interactoption
    (:`Is Valid`
      (`Widget.RemoveFromParent` _interactoption)
      (bind _asgame_controller (cast `/Game/Controllers/GameController` (`GameplayStatics.GetPlayerController` 0)))
      (remove `/Game/Controllers/GameController.StartTheTalk` _asgame_controller (delegate `StartTheMainScript`)))))

(event `StartTheMainScript`
  (`Widget.RemoveFromParent` (`self.InteractOption`))
  (if (not (`self.IsGameComplete`))
    ;[1 1 1] gameCharacter
    (`self.createSubtitles`)
    (bind _asbp_ggcharacter (cast `/Game/BP_Characters/BP_GGCharacter` (`GameplayStatics.GetPlayerCharacter` 0)))
    (`self.DisableInput` _asbp_ggcharacter null)
    (bind _asgame_controller (cast `/Game/Controllers/GameController` (`GameplayStatics.GetPlayerController` 0)))
    (set `self.As Game Controller` _asgame_controller)
    (`/Game/Controllers/GameController.CinematicStart` _asgame_controller)
    (`self.Next Cutscene` false)
    (add `/Game/Controllers/GameController.PressToContinue` _asgame_controller (delegate `PressToContinue_Event`))
    (else
      (`self.createSubtitles`)
      (bind _asgame_controller_2 (cast `/Game/Controllers/GameController` (`GameplayStatics.GetPlayerController` 0)))
      (`/Game/Controllers/GameController.CinematicStart` _asgame_controller_2)
      (`self.ShowNextLine` "/Game/TextInGame/CompleteText.CompleteText")
      (add `/Game/Controllers/GameController.PressToContinue` _asgame_controller_2 (delegate `CompleteDialog`)))))

(event `SetTimer`
  (`/Game/UI/WB_Quize.StartTimer` (`self.QuizeRef`))
  (bind _asgame_controller (cast `/Game/Controllers/GameController` (`GameplayStatics.GetPlayerController` 0)))
  (add `/Game/Controllers/GameController.BadEndingStart` _asgame_controller (delegate `EndQuiz`)))

(event `Finished anim`
  ;[1 1 1] Цикл катсцены
  (if (`self.IsQuizOn`)
    (if (!= (`KismetArrayLibrary.Array_Length` (`self.LoopCollection`)) (+ (`self.LoopQueue`) 1))
      ;[1 1 1] nextCutscene
      (bind _result (`/Engine/EditorBlueprintResources/StandardMacros.IncrementInt` (`self.LoopQueue`))
        (:`  `
          (set `self.LoopQueue` _result)
          (bind _result_2 (`/Engine/EditorBlueprintResources/StandardMacros.IncrementInt` (`self.SequenceCutsceneNum`))
            (:`  `
              (set `self.SequenceCutsceneNum` _result_2)
              (bind _result_3 (`/Engine/EditorBlueprintResources/StandardMacros.IncrementInt` (`self.CurrentText`))
                (:`  `
                  (set `self.CurrentText` _result_3)
                  (`/Game/UI/WB_Subtitles.EmptyText` (`self.SubtitlesWidgetRef`))
                  (`self.Next Cutscene` false)))))))
      (else
        ;[1 1 1] Quize game
        (`self.HideShowTextUI`)
        (bind _asgame_controller (cast `/Game/Controllers/GameController` (`GameplayStatics.GetPlayerController` 0)))
        (`/Game/Controllers/GameController.QuizIsOn` _asgame_controller)
        (`self.CreateQuizWidget`)
        (bind _returnvalue (`AddComponent|NODE_AddAudioComponent-1`))
        (set `self.SoundMusic` _returnvalue)
        (`self.QuizeStarted`)))
    (else
      (`self.EndScene`))))

(event `EndQuiz`
  (`self.AfterQuize`))

(event `PressToContinue_Event`
  ;[1 1 1] Пропуск кат сцены
  (`MovieSceneSequencePlayer.GoToEndAndStop` (`self.Sequence Player`))
  (set `self.Action Button is pressed` true)
  (`self.Finished anim`))

(event `InitScoreResult`
  ;[1 1 1] InitScoreResult
  (bind _returnvalue (`|CreateWidget` "/Game/UI/WB_ScoreResult.WB_ScoreResult_C"))
  (set `self.ScoreResult ref` _returnvalue)
  (`/Game/UI/WB_ScoreResult.DisplayScoreResult` _returnvalue (`KismetStringLibrary.Conv_IntToString` (`self.Score`)))
  (`UserWidget.AddToViewport` _returnvalue 0))

(event `Showtext`
  (params (IsEnding :type Boolean) (EndingText :type "DataTable Object Reference"))
  ;[1 1 1] show text
  (if IsEnding
    (set `self.TextCollection` EndingText))
  (`self.ShowNextLine` (`self.TextCollection`)))

(event `CompleteDialog`
  (`self.HideText`)
  (`/Game/Controllers/GameController.CinematicEnd` (stale `StartTheMainScript` _asgame_controller_2)))

(event `QuizeStarted`
  ;[1 1 1] QuizeGame
  (`self.Next Question` false))

(event `CreateQuizWidget`
  (bind _returnvalue (`GameplayStatics.GetPlayerController` 0))
  ;[1 1 1] QuizeWidget
  (bind _returnvalue_2 (`|CreateWidget` "/Game/UI/WB_Quize.WB_Quize_C"))
  (bind _output_get (set `self.QuizeRef` _returnvalue_2))
  (`UserWidget.AddToViewport` _output_get 0)
  (`WidgetBlueprintLibrary.SetInputMode_GameAndUIEx` _returnvalue null)
  (set `PlayerController.bShowMouseCursor` true _returnvalue))

(event `createSubtitles`
  ;[1 1 1] Subtitles display
  (bind _returnvalue (`|CreateWidget` "/Game/UI/WB_Subtitles.WB_Subtitles_C"))
  (bind _output_get (set `self.SubtitlesWidgetRef` _returnvalue))
  (`UserWidget.AddToViewport` _output_get 0)
  (`self.ClearSubtitles`))

(event `self.Next Question`
  (params (IsAnswerCorrect :type Boolean))
  (bind _question (`self.Question`))
  (bind _currentquestion (`self.CurrentQuestion`))
  (bind _quizeref (`self.QuizeRef`))
  ;[1 1 1] QuizeGame
  (`/Game/UI/WB_Quize.DisplayCuurrentQuestion` (`self.QuizeRef`) (`KismetStringLibrary.Conv_IntToString` (`KismetArrayLibrary.Array_Length` _question)) (`KismetStringLibrary.Conv_IntToString` (+ (`self.CurrentQuestion`) 1)))
  (if IsAnswerCorrect
    (bind _result (`/Engine/EditorBlueprintResources/StandardMacros.IncrementInt` (`self.Score`))
      (:`  `
        (`/Game/UI/WB_Quize.DisplayNewScore` (`self.QuizeRef`) (`KismetStringLibrary.Conv_IntToString` _result)))))
  (if (> (+ (`KismetArrayLibrary.Array_LastIndex` _question) 1) (`self.CurrentQuestion`))
    (`/Game/UI/WB_Quize.ClearStyle` _quizeref)
    (`/Game/UI/WB_Quize.InitQuestion` _quizeref (`|GetArrayItem` (`self.Question`) _currentquestion))
    (`self.SetTimer`)
    (`/Engine/EditorBlueprintResources/StandardMacros.IncrementInt` _currentquestion)
    (else
      (`/Game/UI/WB_Quize.ClearTimer` (`self.QuizeRef`))
      (`self.AfterQuize`))))

(event `AfterQuize`
  ;[1 1 1] AfterQuize
  (set `self.IsQuizOn` false)
  (`/Game/UI/WB_Quize.DestroyQuize` (`self.QuizeRef`))
  (`self.InitScoreResult`)
  (bind _asgame_controller (cast `/Game/Controllers/GameController` (`GameplayStatics.GetPlayerController` 0)))
  (add `/Game/Controllers/GameController.ExitFromScore` _asgame_controller (delegate `ScoreResultExit`)))

(event `EndScene`
  ;[1 1 1] End of scene
  (bind _asgame_controller (cast `/Game/Controllers/GameController` (`GameplayStatics.GetPlayerController` 0)))
  (remove `/Game/Controllers/GameController.PressToContinue` _asgame_controller (delegate `PressToContinue_Event`))
  (`/Game/Controllers/GameController.CinematicEnd` _asgame_controller)
  (`self.HideText`)
  ;;[1 1 1] ToZero
  (set `self.TextCollection` "/Game/TextInGame/scene_2.scene_2")
  (set `self.LoopQueue` 0)
  (set `self.SequenceCutsceneNum` 0)
  (set `self.CurrentQuestion` 0)
  (set `self.Score` 0)
  (set `self.CurrentText` 0)
  (set `self.IsQuizOn` true)
  (set `self.Is Ending` false)
  (bind _asbp_ggcharacter (cast `/Game/BP_Characters/BP_GGCharacter` (`GameplayStatics.GetPlayerCharacter` 0)))
  (`self.EnableInput` _asbp_ggcharacter null))

(event `ScoreResultExit`
  (bind _returnvalue (`GameplayStatics.GetPlayerController` 0))
  ;[1 1 1] AfterQuize
  (set `PlayerController.bShowMouseCursor` false _returnvalue)
  (`WidgetBlueprintLibrary.SetInputMode_GameOnly` _returnvalue)
  (bind _asgame_controller (cast `/Game/Controllers/GameController` (`GameplayStatics.GetPlayerController` 0)))
  (`/Game/Controllers/GameController.QuizisOff` _asgame_controller)
  (`AudioComponent.Stop` (`self.SoundMusic`))
  (`self.ContinueToEnd`))

(event `ClearSubtitles`
  ;[1 1 1] Subtitles display
  (`/Game/UI/WB_Subtitles.DisplayLine` (`self.SubtitlesWidgetRef`) "" ""))

(event `hideTextBox_Event`
  ;[1 1 1] Subtitles display
  (`Widget.RemoveFromParent` (`self.SubtitlesWidgetRef`)))

(event `ContinueToEnd`
  ;[1 1 1] QuizeGame
  (if (>= (`self.Score`) (+ (/ (`self.CurrentQuestion`) 2) 1))
    (`self.goodEnding`)
    (else
      (`self.BadEnding`))))

(event `BadEnding`
  ;[1 1 1] BadEnding
  (`self.createSubtitles`)
  (bind _outactor (`LevelSequencePlayer.CreateLevelSequencePlayer` (`self.BadEndingCatscene`)))
  (set `self.CurrentText` 0)
  (set `self.Is Ending` true)
  (`self.Showtext` (`self.Is Ending`) "/Game/TextInGame/BadEnding_Quiz1.BadEnding_Quiz1")
  (set `self.EndingSequence Player` _outactor)
  (`self.PlayEnding` (`self.EndingSequence Player`) -1 :!label _label_2))

(event `ShowNextLine`
  (params (NarrationList :type "DataTable Object Reference"))
  (bind _currentnarrationlist (`self.CurrentNarrationList`))
  ;[1 1 1] Subtitles display
  (set `self.CurrentNarrationList` NarrationList)
  (bind _outrownames (`DataTableFunctionLibrary.GetDataTableRowNames` _currentnarrationlist))
  (bind _returnvalue (`|GetDataTableRow` _currentnarrationlist (`|GetArrayItem` _outrownames (`self.CurrentText`)))
    (:`then`
      (bind (_linetoshow _namecharacter) (break `/Game/TextInGame/SubtitlesStruct` _returnvalue))
      (`/Game/UI/WB_Subtitles.DisplayLine` (`self.SubtitlesWidgetRef`) _linetoshow _namecharacter))))

(event `HideText`
  ;[1 1 1] Subtitles display
  (`Widget.RemoveFromParent` (`self.SubtitlesWidgetRef`)))

(event `PlayEnding`
  (params (SequencePlayer :type "LevelSequenceActor Object Reference") (Islooping :type Integer))
  ;[1 1 1] PlayEnding
  (`self.Next Cutscene` true SequencePlayer Islooping))

(event `HideShowTextUI`
  ;[1 1 1] Subtitles display
  (`/Game/UI/WB_Subtitles.Hide/showUI` (`self.SubtitlesWidgetRef`)))

(event `goodEnding`
  ;[1 1 1] Good ending
  (`self.SavePoints`)
  (`self.createSubtitles`)
  (bind _outactor (`LevelSequencePlayer.CreateLevelSequencePlayer` (`self.GoodEndingCatscene`)))
  (set `self.CurrentText` 0)
  (set `self.Is Ending` true)
  (`self.Showtext` (`self.Is Ending`) "/Game/TextInGame/GoodEnding_Quiz1.GoodEnding_Quiz1")
  (set `self.EndingSequence Player` _outactor)
  (set `self.IsGameComplete` true)
  (goto _label_2))

(event `SavePoints`
  ;[1 1 1] not for first level
  (bind _returnvalue (`GameplayStatics.LoadGameFromSlot` (`self.Slot Name`)))
  (bind _assave_progress (cast `/Game/Blueprints/SaveProgress` _returnvalue))
  (`/Engine/EditorBlueprintResources/StandardMacros.IncrementInt` (`/Game/Blueprints/SaveProgress.Points` _assave_progress)
    (:`  `
      (set `/Game/Blueprints/SaveProgress.IsNeedRestart` false _assave_progress)
      (`GameplayStatics.SaveGameToSlot` _assave_progress (`self.Slot Name`)))))

(event `self.NameBox.OnComponentBeginOverlap`
  (params (OverlappedComponent :type "PrimitiveComponent Object Reference") (OtherActor :type "Actor Object Reference") (OtherComp :type "PrimitiveComponent Object Reference") (OtherBodyIndex :type Integer) (bFromSweep :type Boolean) (SweepResult :type "HitResult Structure (by ref)"))
  (`SceneComponent.SetHiddenInGame` (`self.TextRender`) false false))

(event `self.NameBox.OnComponentEndOverlap`
  (params (OverlappedComponent :type "PrimitiveComponent Object Reference") (OtherActor :type "Actor Object Reference") (OtherComp :type "PrimitiveComponent Object Reference") (OtherBodyIndex :type Integer))
  (`SceneComponent.SetHiddenInGame` (`self.TextRender`) true false))

(fn `UserConstructionScript`)